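; Timer component for a stimulus test that plays repeating visual, audio, haptic or visual-audio impulses while timing a run.
; On BeginPlay, TestType selects the fast or slow interval and impulse type, and the component binds to BP_TestGameMode's timer start/end events.
; A looping timer toggles all point light intensities, plays a tick sound or triggers game mode vibration.
; On end, it saves elapsed seconds under the test type name.
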(event Custom|커스텀이벤트
  (CallFunction|PlayImpulse))

(event Custom|TimerStartEvent_이벤트
  (if (not (Variables|Temp|GetisTImerRunning))
    (CallFunction|TimerStart)
    (CallFunction|PlayImpulse)
    (bind _returnvalue (Utilities|Time|SetTimerbyEvent (delegate Custom|커스텀이벤트) (Variables|Temp|GetTimePercent) true))
    (Variables|Temp|SetTimer _returnvalue)))

(event Custom|TimerEndEvent_이벤트
  (if (Variables|Temp|GetisTImerRunning)
    (CallFunction|TimerEnd)
    (Utilities|Time|ClearandInvalidateTimerbyHandle (Variables|Temp|GetTimer))))

(event EventBeginPlay
  (Utilities|FlowControl|Sequence
    (:then_0
      (switch Utilities|FlowControl|Switch|SwitchonTestType (Variables|Enum|GetTestType)
        (:NewEnumerator0
          (Variables|Temp|SetTimePercent (Variables|Default|GetFastPercent) :!label _label))
        (:NewEnumerator1
          (Variables|Temp|SetTimePercent (Variables|Default|GetSlowPercent) :!label _label_2))
        (:NewEnumerator2
          (goto _label))
        (:NewEnumerator3
          (goto _label_2))
        (:NewEnumerator4
          (goto _label))
        (:NewEnumerator5
          (goto _label_2))
        (:NewEnumerator6
          (goto _label))
        (:NewEnumerator7
          (goto _label_2))
        (:NewEnumerator8
          _)
        (:NewEnumerator9
          _))
      (switch Utilities|FlowControl|Switch|SwitchonTestType (Variables|Enum|GetTestType)
        (:NewEnumerator0
          (Variables|Enum|SetImpulseType "NewEnumerator0" :!label _label_3))
        (:NewEnumerator1
          (goto _label_3))
        (:NewEnumerator2
          (Variables|Enum|SetImpulseType "NewEnumerator1" :!label _label_4))
        (:NewEnumerator3
          (goto _label_4))
        (:NewEnumerator4
          (Variables|Enum|SetImpulseType "NewEnumerator2" :!label _label_5))
        (:NewEnumerator5
          (goto _label_5))
        (:NewEnumerator6
          (Variables|Enum|SetImpulseType "NewEnumerator3" :!label _label_6))
        (:NewEnumerator7
          (goto _label_6))
        (:NewEnumerator8
          (Variables|Enum|SetImpulseType "NewEnumerator4" :!label _label_7))
        (:NewEnumerator9
          (goto _label_7))))
    (:then_1
      (bind _asbp_test_game_mode (Utilities|Casting|CastToBP_TestGameMode (Game|GetGameMode)))
      (Variables|Temp|SetAs%20BP%20Test%20Game%20Mode _asbp_test_game_mode))
    (:then_2
      (bind _outactors (Actor|GetAllActorsOfClass "/Script/Engine.PointLight"))
      (Variables|Temp|Setlights%20array _outactors))
    (:then_3
      (EventDispatchers|AssignTimerStartEvent (Variables|Temp|GetAs%20BP%20Test%20Game%20Mode) (delegate Custom|TimerStartEvent_이벤트))
      (EventDispatchers|AssignTimerEndEvent (Variables|Temp|GetAs%20BP%20Test%20Game%20Mode) (delegate Custom|TimerEndEvent_이벤트)))))

(event EventTick
  (params (DeltaSeconds :type Float%20%28single-precision%29))
  (Variables|Temp|SetTime (+ DeltaSeconds (Variables|Temp|GetTime))))

(fn PlayImpulse
  (switch Utilities|FlowControl|Switch|SwitchonImpuleType (Variables|Enum|GetImpulseType)
    (:NewEnumerator0
      (CallFunction|PlayVisual))
    (:NewEnumerator1
      (CallFunction|PlaySound))
    (:NewEnumerator2
      (CallFunction|PlayVibration))
    (:NewEnumerator3
      (CallFunction|PlayVisual)
      (CallFunction|PlaySound))))

(fn PlaySound
  (Audio|PlaySoundatLocation (Variables|Default|GetTickSound) (Transformation|GetActorLocation (Components|GetOwner)) "0, 0, 0" 3.0 1.0 0.0 0 0 0 0))

(fn PlayVibration
  (Default|CallVibration (Variables|Temp|GetAs%20BP%20Test%20Game%20Mode)))

(fn PlayVisual
  (for _array_element (Variables|Temp|Getlights%20array)
    (if (>= (Variables|/Script/Engine.LightComponentBase|GetIntensity (Variables|/Script/Engine.PointLight|GetPointLightComponent _array_element)) 15.0)
      (Rendering|Components|Light|SetIntensity (Variables|/Script/Engine.PointLight|GetPointLightComponent _array_element) 5.0)
      (else
        (Rendering|Components|Light|SetIntensity (Variables|/Script/Engine.PointLight|GetPointLightComponent _array_element) 2e+01)))))

(fn TimerStart
  (Variables|Temp|SetisTImerRunning true)
  (Variables|Temp|SetTimerStartTime (Variables|Temp|GetTime)))

(fn TimerEnd
  (bind _as_bp_test_game_mode (Variables|Temp|GetAs%20BP%20Test%20Game%20Mode))
  (Variables|Temp|SetisTImerRunning false)
  (Variables|Temp|SetTimerEndTime (Variables|Temp|GetTime))
  (Default|SaveSecondData _as_bp_test_game_mode (Utilities|String|EnumtoString (Variables|Enum|GetTestType)) (- (Variables|Temp|GetTimerEndTime) (Variables|Temp|GetTimerStartTime)))
  (Default|PrintSaveDataMap _as_bp_test_game_mode))