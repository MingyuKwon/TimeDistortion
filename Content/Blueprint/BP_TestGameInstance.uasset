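; BP_TestGameInstance is a test game instance that stores timing results in seconds from a default run and two test runs.
; SetTestSecond saves the incoming value to Second, then writes it to the first negative slot among Default30Second, Test130Second and Test230Second, treating negative as unset.
; Each stored value is printed to screen, and once all three slots are filled it prints that testing is already done.
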(fn SetTestSecond
  (params (TestSecond :type Float%20%28double-precision%29))
  (LocalVariables|SetSecond TestSecond)
  (if (< (Variables|Default|GetDefault_30Second) 0.0)
    (bind _output_get (Variables|Default|SetDefault_30Second (LocalVariables|GetSecond)))
    (Development|PrintString (Utilities|String|ToString(Float) _output_get) true true "(R=0.000000,G=0.660000,B=1.000000,A=1.000000)" 5.0)
    (elif (< (Variables|Default|GetTest1_30Second) 0.0)
      (bind _output_get_2 (Variables|Default|SetTest1_30Second (LocalVariables|GetSecond)))
      (Development|PrintString (Utilities|String|ToString(Float) _output_get_2) true true "(R=0.000000,G=0.660000,B=1.000000,A=1.000000)" 5.0)
      (elif (< (Variables|Default|GetTest2_30Second) 0.0)
        (bind _output_get_3 (Variables|Default|SetTest2_30Second (LocalVariables|GetSecond)))
        (Development|PrintString (Utilities|String|ToString(Float) _output_get_3) true true "(R=0.000000,G=0.660000,B=1.000000,A=1.000000)" 5.0)
        (else
          (Development|PrintString "Test has Alerady Done two times"))))))