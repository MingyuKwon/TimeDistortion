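; BP_ColorText is an actor that displays three color-named text panels (Red, Green, Blue) through widget components.
; On BeginPlay it casts each component's user widget to WBP_AnnouncePanel and sets it to the matching RedText, GreenText or BlueText variable.
; The casts run in sequence, so a failed cast leaves the remaining panels unset.
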(event EventBeginPlay
  (bind _aswbp_announce_panel (Utilities|Casting|CastToWBP_AnnouncePanel (UserInterface|GetUserWidgetObject (Variables|Default|GetRed))))
  (Default|SetText _aswbp_announce_panel (Variables|Default|GetRedText))
  (bind _aswbp_announce_panel_2 (Utilities|Casting|CastToWBP_AnnouncePanel (UserInterface|GetUserWidgetObject (Variables|Default|GetGreen))))
  (Default|SetText _aswbp_announce_panel_2 (Variables|Default|GetGreenText))
  (bind _aswbp_announce_panel_3 (Utilities|Casting|CastToWBP_AnnouncePanel (UserInterface|GetUserWidgetObject (Variables|Default|GetBlue))))
  (Default|SetText _aswbp_announce_panel_3 (Variables|Default|GetBlueText)))

(event Collision|EventActorBeginOverlap
  (params (OtherActor :type Actor%20Object%20Reference)))

(event EventTick
  (params (DeltaSeconds :type Float%20%28single-precision%29)))

(fn ConstructionScript)