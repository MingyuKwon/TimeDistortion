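; BP_AnnounceText is an actor that shows an announcement on a WBP_AnnouncePanel widget, with text chosen by the current level.
; On BeginPlay it caches the panel from its Text widget component, then switches on the current level name.
; Each Fast and Slow room pair shares one message for visual, sound, visual-sound or touch.
; Any other level falls back to DefaultText through SetDefaultText.
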(event EventBeginPlay
  (bind _aswbp_announce_panel (Utilities|Casting|CastToWBP_AnnouncePanel (UserInterface|GetUserWidgetObject (Variables|Default|GetText))))
  (Variables|Default|SetAs%20WBP%20Announce%20Panel _aswbp_announce_panel)
  (bind _returnvalue (Game|GetCurrentLevelName true))
  (switch string _returnvalue
    (:Default
      (CallFunction|SetDefaultText))
    (:VisualFastRoom
      (Variables|Default|SetShowText (Variables|Default|GetVisualText) :!label _label)
      (Default|SetText (Variables|Default|GetAs%20WBP%20Announce%20Panel) (Variables|Default|GetShowText) :!label _label_2))
    (:VisualSlowRoom
      (goto _label))
    (:SoundFastRoom
      (Variables|Default|SetShowText (Variables|Default|GetSoundlText) :!label _label_3)
      (goto _label_2))
    (:SoundSlowRoom
      (goto _label_3))
    (:VisualSoundFastRoom
      (Variables|Default|SetShowText (Variables|Default|GetVisualSoundText) :!label _label_4)
      (goto _label_2))
    (:VisualSoundSlowRoom
      (goto _label_4))
    (:TouchFastRoom
      (Variables|Default|SetShowText (Variables|Default|GetTouchlText) :!label _label_5)
      (goto _label_2))
    (:TouchSlowRoom
      (goto _label_5))))

(event Collision|EventActorBeginOverlap
  (params (OtherActor :type Actor%20Object%20Reference)))

(event EventTick
  (params (DeltaSeconds :type Float%20%28single-precision%29)))

(fn ConstructionScript)

(fn SetDefaultText
  (Default|SetText (Variables|Default|GetAs%20WBP%20Announce%20Panel) (Variables|Default|GetDefaultText)))