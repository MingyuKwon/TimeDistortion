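; BP_Timer is a test timer actor that counts up to TestTime and displays it on a WBP_AnnouncePanel widget.
; Tick accumulates time scaled by ChangePercent, with a separate accumulator flagging each whole scaled second.
; While the timer is available, optional visual, sound and touch feedback update the text, play a tick or request vibration through BP_TestGameMode.
; On reaching TestTime, it stops feedback and tells the game mode to enable the button.
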(event EventBeginPlay
  (bind _aswbp_announce_panel (Utilities|Casting|CastToWBP_AnnouncePanel (UserInterface|GetUserWidgetObject (Variables|Default|GetTimer))))
  (bind _output_get (Variables|Default|SetAs%20WBP%20Announce%20Panel _aswbp_announce_panel))
  (Default|SetTextColor _output_get (Variables|Settable|GetTextColor))
  (bind _asbp_test_game_mode (Utilities|Casting|CastToBP_TestGameMode (Game|GetGameMode)))
  (Variables|Default|SetAs%20BP%20Test%20Game%20Mode _asbp_test_game_mode))

(event Collision|EventActorBeginOverlap
  (params (OtherActor :type Actor%20Object%20Reference)))

(event EventTick
  (params (DeltaSeconds :type Float%20%28single-precision%29))
  (CallFunction|SetSecond DeltaSeconds)
  (CallFunction|SetTimeSecond)
  (if (Variables|Default|GetisTimerAvailable)
    (CallFunction|SetVisual)
    (CallFunction|SetSound)
    (CallFunction|SetTouch)
    (Variables|Default|SetisNowTimeSecondAwake false)
    (CallFunction|IsNowTimerEnd (Variables|Default|GetSecond))))

(fn ConstructionScript)

(fn FloattoString
  (params (Second :type Float%20%28double-precision%29))
  (bind _output_get (LocalVariables|SetLocalSecond Second))
  (LocalVariables|SetFront (Class|KismetMathLibrary|ToInt64(Float) _output_get))
  (bind _output_get_2 (LocalVariables|SetBack (- (LocalVariables|GetLocalSecond) (Math|Conversions|ToFloat(Integer) (LocalVariables|GetFront)))))
  (return (Utilities|String|Append (Utilities|String|Append (Utilities|String|ToString(Integer) (LocalVariables|GetFront)) ":") (Utilities|String|ToString(Integer) (Class|KismetMathLibrary|ToInt64(Float) (* _output_get_2 1e+02))))))

(fn IsNowTimerEnd
  (params (A :type Float%20%28double-precision%29))
  (if (>= A (Variables|Default|GetTestTime))
    (Variables|Default|SetisTimerAvailable false)
    (bind _as_bp_test_game_mode (Variables|Default|GetAs%20BP%20Test%20Game%20Mode)
      (:then
        (Default|CallButtonEnableEvent _as_bp_test_game_mode true))
      (:else))))

(fn SetSecond
  (params (A :type Float%20%28double-precision%29))
  (bind _changepercent (Variables|Settable|GetChangePercent))
  (bind _returnvalue (* A _changepercent))
  (Variables|Default|SetSoundSecond (+ _returnvalue (Variables|Default|GetSoundSecond)))
  (Variables|Default|SetSecond (Math|Float|Clamp(Float) (+ (Variables|Default|GetSecond) _returnvalue) 0.0 (Variables|Default|GetTestTime))))

(fn SetVisual
  (if (Variables|Settable|GetisVisual)
    (bind _as_wbp_announce_panel (Variables|Default|GetAs%20WBP%20Announce%20Panel)
      (:then
        (bind _out (CallFunction|FloattoString (Variables|Default|GetSecond)))
        (Default|SetText _as_wbp_announce_panel _out))
      (:else))
    (else
      (bind _as_wbp_announce_panel_2 (Variables|Default|GetAs%20WBP%20Announce%20Panel)
        (:then
          (Default|SetText _as_wbp_announce_panel_2))
        (:else)))))

(fn SetSound
  (if (Variables|Settable|GetisSound)
    (if (Variables|Default|GetisNowTimeSecondAwake)
      (Audio|PlaySoundatLocation (Variables|Settable|GetTickSound) (Transformation|GetActorLocation self) "0, 0, 0" 3.0 1.0 0.0 0 0 0 0))))

(fn SetTouch
  (if (Variables|Settable|GetisTouch)
    (if (Variables|Default|GetisNowTimeSecondAwake)
      (Default|CallVibration (Variables|Default|GetAs%20BP%20Test%20Game%20Mode)))))

(fn SetTimeSecond
  (if (>= (Variables|Default|GetSoundSecond) 1.0)
    (Variables|Default|SetSoundSecond (- (Variables|Default|GetSoundSecond) 1.0))
    (Variables|Default|SetisNowTimeSecondAwake true)))