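; BP_Warp is a level-exit warp that opens the next stage when something overlaps it, once it has been unlocked.
; On BeginPlay it binds its Warp component's overlap and listens to BP_TestGameMode's ButtonFinishedEvent, which enables the warp.
; An overlap while enabled gets the next stage name from BP_TestGameInstance, opens that level by name, then disables the warp.
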(event Custom|OnComponentBeginOverlap_이벤트
  (params (OverlappedComponent :type Primitive%20Component%20Object%20Reference) (OtherActor :type Actor%20Object%20Reference) (OtherComp :type Primitive%20Component%20Object%20Reference) (OtherBodyIndex :type Integer) (bFromSweep :type Boolean) (SweepResult :type Hit%20Result%20Structure%20%28by%20ref%29))
  (if (Variables|Default|GetWarpEnable)
    (bind _asbp_test_game_instance (Utilities|Casting|CastToBP_TestGameInstance (Game|GetGameInstance)))
    (bind _nextstagename (Default|GetNextStageName _asbp_test_game_instance))
    (Game|OpenLevel(byName) (Utilities|String|StringToName _nextstagename))
    (Variables|Default|SetWarpEnable false)))

(event Custom|ButtonFinishedEvent_이벤트
  (Variables|Default|SetWarpEnable true))

(event EventBeginPlay
  (Collision|AssignOnComponentBeginOverlap (Variables|Default|GetWarp) (delegate Custom|OnComponentBeginOverlap_이벤트))
  (bind _asbp_test_game_mode (Utilities|Casting|CastToBP_TestGameMode (Game|GetGameMode)))
  (EventDispatchers|AssignButtonFinishedEvent _asbp_test_game_mode (delegate Custom|ButtonFinishedEvent_이벤트)))

(event Collision|EventActorBeginOverlap
  (params (OtherActor :type Actor%20Object%20Reference)))

(event EventTick
  (params (DeltaSeconds :type Float%20%28single-precision%29)))

(fn ConstructionScript)