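; Stage-selection actor that displays a stage number and can warp the player into the StartRoom level.
; On BeginPlay it writes StageIndex as text to the WBP_AnnouncePanel in its widget component.
; MovetoStartRoom, not called within this file, checks WarpEnable, stores StageIndex as TestCaseNum in BP_TestGameInstance, then opens StartRoom, carrying the selection across the level load.
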(event EventBeginPlay
  (bind _aswbp_announce_panel (Utilities|Casting|CastToWBP_AnnouncePanel (UserInterface|GetWidget (Variables|Default|GetWidget))))
  (Variables|Default|SetAs%20WBP%20Announce%20Panel _aswbp_announce_panel)
  (Default|SetText (Variables|Default|GetAs%20WBP%20Announce%20Panel) (Utilities|String|ToString(Integer) (Variables|Default|GetStageIndex))))

(event Collision|EventActorBeginOverlap
  (params (OtherActor :type Actor%20Object%20Reference)))

(event EventTick
  (params (DeltaSeconds :type Float%20%28single-precision%29)))

(fn ConstructionScript)

(fn MovetoStartRoom
  (if (Variables|Default|GetWarpEnable)
    (bind _asbp_test_game_instance (Utilities|Casting|CastToBP_TestGameInstance (Game|GetGameInstance)))
    (Variables|/Game/Blueprint/BP_TestGameInstance.BP_TestGameInstance_C|SetTestCaseNum _asbp_test_game_instance (Variables|Default|GetStageIndex))
    (Game|OpenLevel(byName) "StartRoom")))