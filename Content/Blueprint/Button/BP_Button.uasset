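; BP_Button is an overlap-triggered button that times a test between two presses, with sound and haptic feedback on both hands.
; It starts disabled outside StartRoom, where enable changes are ignored, and follows the game mode's ButtonEnableEvent, resetting its state when enabled.
; While available, the first press records a Tick-accumulated start time and the second saves the elapsed seconds to BP_TestGameInstance, with the material showing each state.
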(event Custom|ButtonEnableEvent_이벤트
  (params (Available :type Boolean))
  (CallFunction|SetButtonEnable Available))

(event Custom|OnComponentBeginOverlap_이벤트
  (params (OverlappedComponent :type Primitive%20Component%20Object%20Reference) (OtherActor :type Actor%20Object%20Reference) (OtherComp :type Primitive%20Component%20Object%20Reference) (OtherBodyIndex :type Integer) (bFromSweep :type Boolean) (SweepResult :type Hit%20Result%20Structure%20%28by%20ref%29))
  (if (Variables|Default|GetbAvailable)
    (Variables|Default|SetState (+ (Variables|Default|GetState) 1))
    (CallFunction|PlayVibrationSound)
    (switch int (Variables|Default|GetState)
      (:Default
        (Development|PrintString "이미 측정 완료된 버튼입니다"))
      (:0
        (Rendering|Material|SetMaterial (Variables|Default|GetButtonMesh) 0 (Variables|Default|GetDefaultMaterial)))
      (:1
        (Rendering|Material|SetMaterial (Variables|Default|GetButtonMesh) 0 (Variables|Default|GetPushedMaterial))
        (Variables|Default|SetStartSecond (Variables|Default|GetRealSecond)))
      (:2
        (Rendering|Material|SetMaterial (Variables|Default|GetButtonMesh) 0 (Variables|Default|GetEndMaterial))
        (Variables|Default|SetEndSecond (Variables|Default|GetRealSecond))
        (bind _asbp_test_game_instance (Utilities|Casting|CastToBP_TestGameInstance (Game|GetGameInstance)))
        (Default|SetTestSecond _asbp_test_game_instance (- (Variables|Default|GetEndSecond) (Variables|Default|GetStartSecond)))))))

(event EventBeginPlay
  (Collision|AssignOnComponentBeginOverlap (Variables|Default|GetButton%20Collision) (delegate Custom|OnComponentBeginOverlap_이벤트))
  (CallFunction|SetButtonEnable false)
  (bind _asbp_test_game_mode (Utilities|Casting|CastToBP_TestGameMode (Game|GetGameMode)))
  (bind _output_get (Variables|Default|SetAs%20BP%20Test%20Game%20Mode _asbp_test_game_mode))
  (EventDispatchers|AssignButtonEnableEvent _output_get (delegate Custom|ButtonEnableEvent_이벤트)))

(event Collision|EventActorBeginOverlap
  (params (OtherActor :type Actor%20Object%20Reference)))

(event EventTick
  (params (DeltaSeconds :type Float%20%28single-precision%29))
  (Variables|Default|SetRealSecond (+ (Variables|Default|GetRealSecond) DeltaSeconds)))

(fn ConstructionScript)

(fn SetButtonEnable
  (params (Available :type Boolean))
  (bind _returnvalue (Game|GetCurrentLevelName true))
  (if (Utilities|Enum|NotEqual(Enum) _returnvalue "StartRoom")
    (bind _output_get (Variables|Default|SetbAvailable Available))
    (if _output_get
      (Rendering|Material|SetMaterial (Variables|Default|GetButtonMesh) 0 (Variables|Default|GetDefaultMaterial))
      (Variables|Default|SetState 0)
      (else
        (Rendering|Material|SetMaterial (Variables|Default|GetButtonMesh) 0 (Variables|Default|GetDisableMaterial))))))

(fn PlayVibrationSound
  (bind _returnvalue (Game|GetPlayerController 0))
  (switch int (Variables|Default|GetState)
    (:Default
      (LocalVariables|SetSound "/Engine/VREditor/Sounds/UI/Camera_Shutter.Camera_Shutter" :!label _label))
    (:0
      (goto _label))
    (:1
      (LocalVariables|SetSound "/Engine/EditorSounds/Notifications/CompileFailed.CompileFailed"))
    (:2
      (LocalVariables|SetSound "/Engine/EditorSounds/Notifications/CompileSuccess.CompileSuccess")))
  (Audio|PlaySoundatLocation (LocalVariables|GetSound) (Transformation|GetActorLocation self) "0, 0, 0" 5.0 1.0 0.0 0 0 0 0)
  (Class|PlayerController|PlayHapticEffect _returnvalue "/Game/VRTemplate/Haptics/PistolFireHapticEffect.PistolFireHapticEffect" "Left" 3e+02 false)
  (Class|PlayerController|PlayHapticEffect _returnvalue "/Game/VRTemplate/Haptics/PistolFireHapticEffect.PistolFireHapticEffect" "Right" 3e+02 false))